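; Player bullet actor that flies by projectile movement, shows a Paper2D flipbook and plays a hit effect on contact with enemies.
; The construction script applies variables for flipbook, looping, color, play rate and local-space velocity, so one class covers different bullet looks and speeds.
; When the capsule overlaps an Enemy-tagged actor, it spawns a scaled-down BP_Effect at the bullet's location, without applying damage or destroying the bullet here.
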(event OnComponentBeginOverlap(Capsule)
  (params (OverlappedComponent :type Primitive%20Component%20Object%20Reference) (OtherActor :type Actor%20Object%20Reference) (OtherComp :type Primitive%20Component%20Object%20Reference) (OtherBodyIndex :type Integer) (bFromSweep :type Boolean) (SweepResult :type Hit%20Result%20Structure%20%28by%20ref%29))
  (if (Actor|ActorHasTag OtherActor "Enemy")
    (Game|SpawnActorfromClass "/Game/Player/BP_Effect.BP_Effect_C" (Math|Transform|MakeTransform (Transformation|GetActorLocation) "0, 0, 0" "0.800000,0.800000,0.800000") "Undefined" "MultiplyWithRoot" 0 "/Game/Bullet/Effects/Hit_Effect01/Hit_Effect.Hit_Effect" false "(R=1.000000,G=1.000000,B=1.000000,A=1.000000)" 1.0 0)))

(event EventBeginPlay)

(event Collision|EventActorBeginOverlap
  (params (OtherActor :type Actor%20Object%20Reference)))

(event EventTick
  (params (DeltaSeconds :type Float%20%28single-precision%29)))

(fn ConstructionScript
  (bind _paperflipbook (Variables|Default|GetPaperFlipbook))
  (Sprite|SetFlipbook _paperflipbook (Variables|Default|GetNew%20Flipbook))
  (Components|Timeline|SetLooping _paperflipbook (Variables|Default|GetNew%20Looping))
  (Sprite|SetSpriteColor _paperflipbook (Variables|Default|GetNew%20Color))
  (Components|Timeline|SetPlayRate _paperflipbook (Variables|Default|GetNew%20Rate))
  (Game|Components|ProjectileMovement|SetVelocityinLocalSpace (Variables|Default|GetProjectileMovement) (Variables|Default|GetNew%20Velocity)))