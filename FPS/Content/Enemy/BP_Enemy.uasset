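; BP_Enemy is a sprite-based shooter enemy covering several types and a boss, selected by EmuEnemy with stats from DT_Enemy.
; Some types follow a spline on Tick, while E2 and the boss move by projectile movement, with delay- and timer-driven bullet patterns.
; Shields break only to shoot mode 2, then HP only to mode 1, awarding bullet EXP.
; Killed enemies add score, explode, drop and splash on water.
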(event OnComponentBeginOverlap(CapsuleComponent)
  (params (OverlappedComponent :type Primitive%20Component%20Object%20Reference) (OtherActor :type Actor%20Object%20Reference) (OtherComp :type Primitive%20Component%20Object%20Reference) (OtherBodyIndex :type Integer) (bFromSweep :type Boolean) (SweepResult :type Hit%20Result%20Structure%20%28by%20ref%29))
  ;[1 1 1] The enemy dop to water overlap
  (if (Actor|ActorHasTag OtherActor "LR")
    (bind _output_get (Variables|Default|SetVectorySpeed (Math|Vector|MakeVector (* (.x (Variables|Default|GetVectorySpeed)) -1.0) (.y (Variables|Default|GetVectorySpeed)) (.z (Variables|Default|GetVectorySpeed)))))
    (Variables|/Script/Engine.MovementComponent|SetVelocity (Variables|Default|GetProjectile) _output_get)
    (elif (Actor|ActorHasTag OtherActor "Water")
      (Game|SpawnActorfromClass "/Game/Player/BP_Effect.BP_Effect_C" (Math|Transform|MakeTransform (+ (Transformation|GetActorLocation) "0.000000,0.000000,8.000000") "0, 0, 0" "2.000000,1.000000,2.500000") "Undefined" "MultiplyWithRoot" 0 "/Game/Effects/Splash_1/Splash_1_FB.Splash_1_FB" false "(R=1.000000,G=1.000000,B=1.000000,A=1.000000)" 1.0 0)
      (Utilities|FlowControl|Delay 0.2)
      (Actor|DestroyActor))))

(event OnComponentBeginOverlap(Capsule)
  (params (OverlappedComponent :type Primitive%20Component%20Object%20Reference) (OtherActor :type Actor%20Object%20Reference) (OtherComp :type Primitive%20Component%20Object%20Reference) (OtherBodyIndex :type Integer) (bFromSweep :type Boolean) (SweepResult :type Hit%20Result%20Structure%20%28by%20ref%29))
  ;[1 1 1] The enemy hit the player
  (Utilities|IsValid OtherActor
    (:Is%20Valid
      (if (Actor|ActorHasTag OtherActor "P")
        (Class|IFPlayer|DamagePlayer(Message) OtherActor (Variables|角色|GetATK))))))

(event Custom|Hit%20Flash
  ;[1 1 1] Hit Flash
  (Sprite|SetSpriteColor (Variables|Default|GetSprite) "(R=1.000000,G=0.000000,B=0.000000,A=1.000000)")
  (Utilities|FlowControl|Delay 0.2)
  (Sprite|SetSpriteColor (Variables|Default|GetSprite) "(R=1.000000,G=1.000000,B=1.000000,A=1.000000)"))

(event Custom|E2
  (bind _shootpoint (Variables|Default|GetShootPoint))
  (bind _shootpoint_2 (Variables|Default|GetShootPoint))
  (bind _returnvalue (Transformation|GetWorldRotation _shootpoint))
  (bind _returnvalue_2 (Transformation|GetWorldRotation _shootpoint_2))
  ;[1 1 1] E2
  (bind _returnvalue_3 (AddComponent|AddProjectileMovementComponent))
  (bind _output_get (Variables|Default|SetProjectile _returnvalue_3))
  (Variables|/Script/Engine.ProjectileMovementComponent|SetProjectileGravityScale _output_get 0.0)
  (Variables|/Script/Engine.MovementComponent|SetVelocity _output_get (select (Variables|Default|GetRight?) (Math|Vector|MakeVector (* (Variables|角色|GetSpeed) 1.0) 0.0 0.0) (Math|Vector|MakeVector (* (Variables|角色|GetSpeed) -1.0) 0.0 0.0)))
  (Utilities|FlowControl|Delay 3.0)
  (Variables|/Script/Engine.MovementComponent|SetVelocity (Variables|Default|GetProjectile) "0, 0, 0")
  (Utilities|FlowControl|Delay 0.5)
  (Variables|Default|SetShootCounts 8)
  (Game|SpawnActorfromClass "/Game/Enemy/BP_Enemy_Bullet_1.BP_Enemy_Bullet_1_C" (Math|Transform|MakeTransform (Transformation|GetWorldLocation _shootpoint_2) (Math|Rotator|MakeRotator (.roll _returnvalue_2) (+ (.pitch _returnvalue_2) (Math|Random|RandomFloatinRange -45.0 45.0)) (.yaw _returnvalue_2)) "1.000000,1.000000,1.000000") "AlwaysSpawn" "MultiplyWithRoot" 0 "(R=1.000000,G=1.000000,B=1.000000,A=1.000000)" "400.000000,0.000000,0.000000" (Variables|角色|GetATK) 1e+01 true 0 :!label _label)
  (bind _result (Math|Integer|DecrementInt (Variables|Default|GetShootCounts))
    (:%20%20
      (if (== _result 0)
        (Utilities|FlowControl|Delay 0.5)
        (Variables|/Script/Engine.MovementComponent|SetVelocity (Variables|Default|GetProjectile) (select (Variables|Default|GetRight?) (Math|Vector|MakeVector (* (Variables|角色|GetSpeed) 1.0) 0.0 0.0) (Math|Vector|MakeVector (* (Variables|角色|GetSpeed) -1.0) 0.0 0.0)))
        (Utilities|FlowControl|Delay 4.0)
        (Variables|/Script/Engine.MovementComponent|SetVelocity (Variables|Default|GetProjectile) "0, 0, 0")
        (bind _output_get_2 (Variables|Default|SetRight? (not (Variables|Default|GetRight?))))
        (Transformation|SetRelativeRotation (Variables|Default|GetSprite) (Math|Rotator|SelectRotator "0.000000,180.000000,0.000000" "0, 0, 0" _output_get_2) false false)
        (Utilities|FlowControl|Delay 0.5)
        (Variables|Default|SetShootCounts 8)
        (Game|SpawnActorfromClass "/Game/Enemy/BP_Enemy_Bullet_1.BP_Enemy_Bullet_1_C" (Math|Transform|MakeTransform (Transformation|GetWorldLocation _shootpoint) (Math|Rotator|MakeRotator (.roll _returnvalue) (+ (.pitch _returnvalue) (Math|Random|RandomFloatinRange -45.0 45.0)) (.yaw _returnvalue)) "1.000000,1.000000,1.000000") "AlwaysSpawn" "MultiplyWithRoot" 0 "(R=1.000000,G=1.000000,B=1.000000,A=1.000000)" "400.000000,0.000000,0.000000" (Variables|角色|GetATK) 1e+01 true 0 :!label _label_2)
        (bind _result_2 (Math|Integer|DecrementInt (Variables|Default|GetShootCounts))
          (:%20%20
            (if (== _result_2 0)
              (Utilities|FlowControl|Delay 0.5)
              (Variables|/Script/Engine.MovementComponent|SetVelocity (Variables|Default|GetProjectile) (select (Variables|Default|GetRight?) (Math|Vector|MakeVector (* (Variables|角色|GetSpeed) 1.0) 0.0 0.0) (Math|Vector|MakeVector (* (Variables|角色|GetSpeed) -1.0) 0.0 0.0)))
              (else
                (Utilities|FlowControl|Delay 0.2)
                (goto _label_2)))))
        (else
          (Utilities|FlowControl|Delay 0.2)
          (goto _label))))))

(event Custom|E3
  ;[1 1 1] E3
  (switch Utilities|FlowControl|Switch|SwitchonEmu_Action (Variables|Default|GetEmu_Action) :!label _label
    (:NewEnumerator0
      _)
    (:NewEnumerator1
      _))
  (Utilities|FlowControl|Delay 1.0)
  (Game|SpawnActorfromClass "/Game/Enemy/BP_Enemy_Bullet_1.BP_Enemy_Bullet_1_C" (Math|Transform|MakeTransform (Transformation|GetWorldLocation (Variables|Default|GetShootPoint)) (Math|Rotator|FindLookatRotation (Transformation|GetActorLocation) (Transformation|GetActorLocation (Game|Player|GetPlayerPawn 0))) "1.000000,1.000000,1.000000") "AlwaysSpawn" "MultiplyWithRoot" 0 "(R=1.000000,G=1.000000,B=1.000000,A=1.000000)" "400.000000,0.000000,0.000000" (Variables|角色|GetATK) 1e+01 true 0)
  (goto _label))

(event Custom|Boss1
  (if (>= (Math|Random|RandomIntegerinRange 0 1) 1)
    (CallFunction|Boss1Mode1)
    (else
      (CallFunction|Boss1Mode2))))

(event Custom|boss_atk_2
  ;[1 1 1] boss mode2
  (Variables|Default|SetShootCounts_II 3)
  (bind _returnvalue (Utilities|Time|SetTimerbyEvent (delegate Custom|Start%20boss1%20mode2%20atk) 0.2 true))
  (Variables|Default|SetStatrtBoss1Mode2AtkHandle _returnvalue))

(event Custom|boss1%20mode%202
  ;[1 1 1] boss mode2
  (Utilities|FlowControl|Delay 1.0)
  (Utilities|Time|SetTimerbyEvent (delegate Custom|boss1%20mode2%20time) 8.0)
  (Variables|Default|GetProjectile
    (:then
      _)
    (:else
      (bind _returnvalue (AddComponent|AddProjectileMovementComponent))
      (bind _output_get (Variables|Default|SetProjectile _returnvalue))
      (Variables|/Script/Engine.ProjectileMovementComponent|SetProjectileGravityScale _output_get 0.0)))
  (bind _output_get_2 (Variables|Default|SetVectorySpeed (* (Variables|角色|GetSpeed) "-1.000000,0.000000,0.000000")))
  (Variables|/Script/Engine.MovementComponent|SetVelocity (Variables|Default|GetProjectile) _output_get_2)
  (Variables|Default|SetShootCounts_II 3)
  (bind _returnvalue_2 (Utilities|Time|SetTimerbyEvent (delegate Custom|Start%20boss1%20mode2%20atk) 0.2 true))
  (Variables|Default|SetStatrtBoss1Mode2AtkHandle _returnvalue_2))

(event Custom|boss1%20mode%201
  (bind _shootpoint (Variables|Default|GetShootPoint))
  (bind _returnvalue (Transformation|GetWorldRotation _shootpoint))
  ;[1 1 1] boss mode1
  (Utilities|FlowControl|Delay 1.0)
  (Variables|Default|SetShootCounts 35)
  (Game|SpawnActorfromClass "/Game/Enemy/BP_Enemy_Bullet_1.BP_Enemy_Bullet_1_C" (Math|Transform|MakeTransform (Transformation|GetWorldLocation _shootpoint) (Math|Rotator|MakeRotator (.roll _returnvalue) (+ (.pitch _returnvalue) (Math|Random|RandomFloatinRange -1.8e+02 1.8e+02)) (.yaw _returnvalue)) "2.000000,2.000000,2.000000") "AlwaysSpawn" "MultiplyWithRoot" 0 "(R=1.000000,G=1.000000,B=1.000000,A=1.000000)" "400.000000,0.000000,0.000000" (Variables|角色|GetATK) 1e+01 true 0 :!label _label)
  (bind _output_get (Variables|Default|SetShootCounts (Math|Integer|Clamp(Integer) (- (Variables|Default|GetShootCounts) 1) 0 99)))
  (if (== _output_get 0)
    (Utilities|FlowControl|Delay 1.0)
    (CallFunction|Boss1)
    (else
      (Utilities|FlowControl|Delay 0.2)
      (goto _label))))

(event Custom|boss1%20mode2%20time
  ;[1 1 1] boss mode2
  (Utilities|FlowControl|Delay 1.0)
  (CallFunction|Boss1)
  (Variables|/Script/Engine.MovementComponent|SetVelocity (Variables|Default|GetProjectile) "0, 0, 0")
  (Variables|Default|SetShootCounts_II 0)
  (Utilities|Time|ClearandInvalidateTimerbyHandle (Variables|Default|GetStatrtBoss1Mode2AtkHandle))
  (Utilities|Time|ClearandInvalidateTimerbyHandle (Variables|Default|Getboss_atk_2_handle)))

(event Custom|Start%20boss1%20mode2%20atk
  (bind _atk (Variables|角色|GetATK))
  ;[1 1 1] boss mode2
  (Game|SpawnActorfromClass "/Game/Enemy/BP_Enemy_Bullet_1.BP_Enemy_Bullet_1_C" (Math|Transform|MakeTransform (Transformation|GetWorldLocation (Variables|Default|GetShootPoint1)) "-90.000000,0.000000,0.000000" "2.000000,2.000000,2.000000") "AlwaysSpawn" "MultiplyWithRoot" 0 "(R=1.000000,G=0.777687,B=0.122004,A=1.000000)" "400.000000,0.000000,0.000000" _atk 1e+01 true 0)
  (Game|SpawnActorfromClass "/Game/Enemy/BP_Enemy_Bullet_1.BP_Enemy_Bullet_1_C" (Math|Transform|MakeTransform (Transformation|GetWorldLocation (Variables|Default|GetShootPoint2)) "-90.000000,0.000000,0.000000" "2.000000,2.000000,2.000000") "AlwaysSpawn" "MultiplyWithRoot" 0 "(R=1.000000,G=0.777687,B=0.122004,A=1.000000)" "400.000000,0.000000,0.000000" _atk 1e+01 true 0)
  (bind _output_get (Variables|Default|SetShootCounts_II (Math|Integer|Clamp(Integer) (- (Variables|Default|GetShootCounts_II) 1) 0 3)))
  (if (== _output_get 0)
    (Utilities|Time|ClearandInvalidateTimerbyHandle (Variables|Default|GetStatrtBoss1Mode2AtkHandle))
    (bind _returnvalue (Utilities|Time|SetTimerbyEvent (EventDispatchers|CreateEvent :!event Custom|boss_atk_2) 2.0))
    (Variables|Default|Setboss_atk_2_handle _returnvalue)))

(event EventBeginPlay
  ;[1 1 1] initialization
  (Utilities|Init))

(event EventDamageEnemy
  (params (Damage :type Float%20%28double-precision%29) (bulletindex :type Emu_PlayerBullet%20Enum :default "NewEnumerator0") (shootmode :type Emu_ShootMode%20Enum :default "NewEnumerator0"))
  ;[1 1 1] Player damage the enemy
  (Utilities|UpdateHp Damage bulletindex shootmode))

(event EventTick
  (params (DeltaSeconds :type Float%20%28single-precision%29))
  ;[1 1 1] Tick
  (switch Utilities|FlowControl|Switch|SwitchonEmu_Enemy (Variables|Character|GetEmu_Enemy)
    (:NewEnumerator0
      _)
    (:NewEnumerator2
      _)
    (:NewEnumerator3
      _))
  (switch Utilities|FlowControl|Switch|SwitchonEmu_Action (Variables|Default|GetEmu_Action)
    (:NewEnumerator0
      _)
    (:NewEnumerator1
      _))
  (bind _output_get (Variables|Default|SetDistance (+ (* DeltaSeconds (Variables|角色|GetSpeed)) (Variables|Default|GetDistance))))
  (Transformation|SetActorLocation (.location (Spline|GetTransformatDistanceAlongSpline (Variables|Default|GetSpline) _output_get "World" false)) false false)
  (switch Utilities|FlowControl|Switch|SwitchonEmu_Enemy (Variables|Character|GetEmu_Enemy)
    (:NewEnumerator2
      _)
    (:NewEnumerator3
      _))
  (Transformation|SetRelativeRotation (Variables|Default|GetSprite) (.rotation (Spline|GetTransformatDistanceAlongSpline (Variables|Default|GetSpline) _output_get "World" false)) false false))

(fn ConstructionScript)