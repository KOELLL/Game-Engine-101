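; Base weapon Blueprint that tracks magazine and reserve ammo and plays the firing animation.
; Fire decrements the current ammo, prints the skeletal mesh's name and plays FireAnimation on it.
; Reload refills the magazine from the reserve; when the reserve cannot exceed the shortfall, the magazine count becomes the reserve count and the reserve drops to zero.
; AmmoCheck reports whether the magazine has rounds, is full, or has reserve left.
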(event EventBeginPlay)

(event Collision|EventActorBeginOverlap
  (params (OtherActor :type Actor%20Object%20Reference)))

(event EventTick
  (params (DeltaSeconds :type Float%20%28single-precision%29)))

(fn ConstructionScript)

(fn Reload
  (LocalVariables|SetLeftAmmo (- (Variables|Ammo|GetCurrentTotalAmmo) (- (Variables|Ammo|GetMaxMagAmmo) (Variables|Ammo|GetCurrentAmmo))))
  (if (<= (- (Variables|Ammo|GetCurrentTotalAmmo) (- (Variables|Ammo|GetMaxMagAmmo) (Variables|Ammo|GetCurrentAmmo))) 0)
    (Variables|Ammo|SetCurrentAmmo (Variables|Ammo|GetCurrentTotalAmmo))
    (Variables|Ammo|SetCurrentTotalAmmo 0)
    (else
      (Variables|Ammo|SetCurrentAmmo (Variables|Ammo|GetMaxMagAmmo))
      (Variables|Ammo|SetCurrentTotalAmmo (LocalVariables|GetLeftAmmo)))))

(fn Fire
  (bind _weaponskm (Variables|Default|GetWeaponSKM))
  (Variables|Ammo|SetCurrentAmmo (- (Variables|Ammo|GetCurrentAmmo) 1))
  (Development|PrintString (Utilities|GetDisplayName _weaponskm))
  (Components|Animation|PlayAnimation _weaponskm (Variables|Presets|GetFireAnimation) false))

(fn AmmoCheck
  (return (> (Variables|Ammo|GetCurrentAmmo) 0) (== (Variables|Ammo|GetCurrentAmmo) (Variables|Ammo|GetMaxMagAmmo)) (> (Variables|Ammo|GetCurrentTotalAmmo) 0)))