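; BP_Player_Bullet is the player's configurable flipbook projectile that damages enemies.
; The construction script applies flipbook, looping, color, play rate, velocity and lifespan from variables.
; Capsule overlaps branch on actor tags: enemies receive a damage message and hit effect, with optional bullet destruction, while walls destroy it and water adds a splash first.
; An older sphere-trace hit check remains unconnected.
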(event OnComponentBeginOverlap(Capsule)
  (params (OverlappedComponent :type Primitive%20Component%20Object%20Reference) (OtherActor :type Actor%20Object%20Reference) (OtherComp :type Primitive%20Component%20Object%20Reference) (OtherBodyIndex :type Integer) (bFromSweep :type Boolean) (SweepResult :type Hit%20Result%20Structure%20%28by%20ref%29))
  ;[1 1 1] To overlap
  (Utilities|IsValid OtherActor
    (:Is%20Valid
      (if (Actor|ActorHasTag OtherActor "E")
        (Class|IFEnemy|DamageEnemy(Message) OtherActor (Variables|Default|GetATK) (Variables|Default|GetBulletIndex) (Variables|Default|GetShootMode))
        (Game|SpawnActorfromClass "/Game/Player/BP_Effect.BP_Effect_C" (Math|Transform|MakeTransform (Transformation|GetActorLocation) "0, 0, 0" "1.000000,1.000000,1.000000") "Undefined" "MultiplyWithRoot" 0 "/Game/Effects/Hit_Effect_1/Hit_Effect_1_FB.Hit_Effect_1_FB" false "(R=1.000000,G=1.000000,B=1.000000,A=1.000000)" 1.0 0)
        (if (Variables|Default|GetDestroy?)
          (Actor|DestroyActor))
        (elif (Actor|ActorHasTag OtherActor "Wall")
          (Actor|DestroyActor)
          (elif (Actor|ActorHasTag OtherActor "Water")
            (Game|SpawnActorfromClass "/Game/Player/BP_Effect.BP_Effect_C" (Math|Transform|MakeTransform (+ (Transformation|GetActorLocation) "0.000000,0.000000,20.000000") "0, 0, 0" "1.000000,1.000000,2.000000") "Undefined" "MultiplyWithRoot" 0 "/Game/Effects/Splash_1/Splash_1_FB.Splash_1_FB" false "(R=1.000000,G=1.000000,B=1.000000,A=1.000000)" 1.0 0)
            (Actor|DestroyActor)))))))

(event EventBeginPlay)

(event Collision|EventActorBeginOverlap
  (params (OtherActor :type Actor%20Object%20Reference)))

(event EventTick
  (params (DeltaSeconds :type Float%20%28single-precision%29)))

(fn ConstructionScript
  (bind _paperflipbook (Variables|Default|GetPaperFlipbook))
  ;[1 1 1] initialization
  (Sprite|SetFlipbook _paperflipbook (Variables|Default|GetNew%20Flipbook))
  (Components|Timeline|SetLooping _paperflipbook (Variables|Default|GetNew%20Looping))
  (Sprite|SetSpriteColor _paperflipbook (Variables|Default|GetNew%20Color))
  (Components|Timeline|SetPlayRate _paperflipbook (Variables|Default|GetNew%20Rate))
  (Variables|/Script/Engine.MovementComponent|SetVelocity (Variables|Default|GetProjectileMovement) (Variables|Default|GetNew%20Velocity))
  (Actor|SetLifeSpan (Variables|Default|GetIn%20Lifespan)))