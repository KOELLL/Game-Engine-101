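; Player character for a 2D plane shooter: Enhanced Input drives movement, firing, bullet switching and wingman rotation.
; Shots combine twin base bullets with the selected type, configured by per-bullet level/EXP maps; the second fire mode spends timer-refilled EP.
; Rewards add score and grant health, bullet types or a timed shield.
; Damage triggers timer-driven flashing invulnerability via collision channels or death at zero HP, with UI_Player mirroring stats.
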(event Custom|Hit%20Flash
  ;[1 1 1] No use Hit Flash
  (Sprite|SetSpriteColor (Variables|Default|GetSprite) "(R=1.000000,G=0.000000,B=0.000000,A=1.000000)")
  (|PlayAnimationOverridewithCallbacks (Variables|Default|GetAs%20ABP%20Player) "/Game/Player/AnimSequences/Player_Hurt.Player_Hurt" "DefaultSlot" 1.0 0.0
    (:then
      (Utilities|FlowControl|Delay 0.2)
      (Sprite|SetSpriteColor (Variables|Default|GetSprite) "(R=1.000000,G=1.000000,B=1.000000,A=1.000000)"))))

(event Custom|Protect
  ;[1 1 1] The player get hurt to open the protect system
  (Utilities|ProtectStart))

(event Custom|FlyScale
  (bind _新建轨道_0 (Timeline|FlyToScale Play)
    (:Update
      (Transformation|SetRelativeScale3D (Variables|Default|GetSprite) (Math|Vector|Lerp(Vector) "3.000000,3.000000,3.000000" "1.000000,1.000000,1.000000" _新建轨道_0)))))

(event Custom|OpenShield
  (bind _capsule (Variables|Default|GetCapsule))
  ;[1 1 1] The player get the reward
  (CallFunction|StartShield false)
  (Collision|SetCollisionResponsetoChannel _capsule "ECC_GameTraceChannel3" "ECR_Ignore")
  (Collision|SetCollisionResponsetoChannel _capsule "ECC_GameTraceChannel4" "ECR_Ignore")
  (Collision|SetCollisionResponsetoChannel _capsule "ECC_GameTraceChannel3" "ECR_Overlap")
  (Collision|SetCollisionResponsetoChannel _capsule "ECC_GameTraceChannel4" "ECR_Overlap"))

(event Input|EnhancedActionEvents|EnhancedInputActionIA_1
  (params (ActionValue :type Boolean) (ElapsedSeconds :type Float%20%28double-precision%29) (TriggeredSeconds :type Float%20%28double-precision%29) (InputAction :type Input%20Action%20Object%20Reference :default "/Game/Player/Input/IA_1.IA_1"))
  ;[1 1 1] Press 1,2,3 to switch the different bullet
  (:Started
    (Utilities|IFBulletActive? "NewEnumerator0")))

(event Input|EnhancedActionEvents|EnhancedInputActionIA_2
  (params (ActionValue :type Boolean) (ElapsedSeconds :type Float%20%28double-precision%29) (TriggeredSeconds :type Float%20%28double-precision%29) (InputAction :type Input%20Action%20Object%20Reference :default "/Game/Player/Input/IA_2.IA_2"))
  ;[1 1 1] Press 1,2,3 to switch the different bullet
  (:Started
    (Utilities|IFBulletActive? "NewEnumerator1")))

(event Input|EnhancedActionEvents|EnhancedInputActionIA_3
  (params (ActionValue :type Boolean) (ElapsedSeconds :type Float%20%28double-precision%29) (TriggeredSeconds :type Float%20%28double-precision%29) (InputAction :type Input%20Action%20Object%20Reference :default "/Game/Player/Input/IA_3.IA_3"))
  ;[1 1 1] Press 1,2,3 to switch the different bullet
  (:Started
    (Utilities|IFBulletActive? "NewEnumerator2")))

(event EventBeginPlay
  ;[1 1 1] Initialization
  (Utilities|Init))

(event EventDamagePlayer
  (params (Damage :type Float%20%28double-precision%29))
  ;[1 1 1] The enemy damage player
  (Utilities|UpdateHp Damage))

(event EventGetReward
  (params (Reward :type Emu_Reward%20Enum :default "NewEnumerator0"))
  ;[1 1 1] The player get the reward
  (CallFunction|UpdateScore (Utilities|Select :Index Reward :NewEnumerator0 350 :NewEnumerator1 500 :NewEnumerator2 500 :NewEnumerator3 500 :NewEnumerator4 450))
  (switch Utilities|FlowControl|Switch|SwitchonEmu_Reward Reward
    (:NewEnumerator0
      (Utilities|UpdateHp -3.0))
    (:NewEnumerator1
      (CallFunction|ActiveBullet "NewEnumerator0"))
    (:NewEnumerator2
      (CallFunction|ActiveBullet "NewEnumerator1"))
    (:NewEnumerator3
      (CallFunction|ActiveBullet "NewEnumerator2"))
    (:NewEnumerator4
      (CallFunction|StartShield true)
      (bind _returnvalue (Utilities|Time|SetTimerbyEvent (delegate Custom|OpenShield) 3.0))
      (Variables|Default|SetShield_Handle _returnvalue))))

(event EventUpdateUIScore
  ;[1 1 1] Update the play score
  (bind _ui_player (Variables|Default|GetUI_Player)
    (:then
      (Default|UpdateUIScore _ui_player))
    (:else)))

(event EventUpdateExpBullet
  (params (bullet :type Emu_PlayerBullet%20Enum :default "NewEnumerator0"))
  ;[1 1 1] Update bullet exp and the level
  (CallFunction|UpdateBulletExpandLevel bullet))

(event OnComponentBeginOverlap(Box)
  (params (OverlappedComponent :type Primitive%20Component%20Object%20Reference) (OtherActor :type Actor%20Object%20Reference) (OtherComp :type Primitive%20Component%20Object%20Reference) (OtherBodyIndex :type Integer) (bFromSweep :type Boolean) (SweepResult :type Hit%20Result%20Structure%20%28by%20ref%29))
  ;[1 1 1] Box Overlap
  (Development|SetHiddeninGame (Variables|Default|GetSplash) false false))

(event OnComponentEndOverlap(Box)
  (params (OverlappedComponent :type Primitive%20Component%20Object%20Reference) (OtherActor :type Actor%20Object%20Reference) (OtherComp :type Primitive%20Component%20Object%20Reference) (OtherBodyIndex :type Integer))
  ;[1 1 1] Box Overlap
  (Development|SetHiddeninGame (Variables|Default|GetSplash) true false))

(event Custom|RefreshEp
  (bind _ep_max (Variables|角色|GetEP_MAX))
  ;[1 1 1] Shoot
  (bind _output_get (Variables|角色|SetEP (Math|Float|Clamp(Float) (+ (Variables|角色|GetEP) 0.5) 0.0 _ep_max)))
  (Default|UpdateUIEp (Variables|Default|GetUI_Player) (/ (Variables|角色|GetEP) (Variables|角色|GetEP_MAX)))
  (if (== _output_get _ep_max)
    (Utilities|Time|ClearandInvalidateTimerbyHandle (Variables|Default|GetRefreshEp_Handle))))

(event Input|EnhancedActionEvents|EnhancedInputActionIA_Move
  (params (ActionValue :type Vector%202D%20Structure) (ElapsedSeconds :type Float%20%28double-precision%29) (TriggeredSeconds :type Float%20%28double-precision%29) (InputAction :type Input%20Action%20Object%20Reference :default "/Game/Player/Input/IA_Move.IA_Move"))
  (bind (_x _y) (Math|Vector2D|BreakVector2D ActionValue))
  ;[1 1 1] Move
  (:Triggered
    (Pawn|Input|AddMovementInput "1.000000,0.000000,0.000000" _x false)
    (Pawn|Input|AddMovementInput "0.000000,0.000000,1.000000" _y false)
    (if (== _y 1.0)
      (bind _output_get (Variables|角色|SetEmu_Fly "NewEnumerator1"))
      (Variables|/Game/Player/ABP_Player.ABP_Player_C|SetEmu_Fly (Variables|Default|GetAs%20ABP%20Player) _output_get)
      (elif (== _y -1.0)
        (bind _output_get_2 (Variables|角色|SetEmu_Fly "NewEnumerator2"))
        (Variables|/Game/Player/ABP_Player.ABP_Player_C|SetEmu_Fly (Variables|Default|GetAs%20ABP%20Player) _output_get_2)
        (else
          (bind _output_get_3 (Variables|角色|SetEmu_Fly "NewEnumerator0"))
          (Variables|/Game/Player/ABP_Player.ABP_Player_C|SetEmu_Fly (Variables|Default|GetAs%20ABP%20Player) _output_get_3)))))
  (:Completed
    (bind _output_get_4 (Variables|角色|SetEmu_Fly "NewEnumerator0"))
    (Variables|/Game/Player/ABP_Player.ABP_Player_C|SetEmu_Fly (Variables|Default|GetAs%20ABP%20Player) _output_get_4)))

(event Input|EnhancedActionEvents|EnhancedInputActionIA_Shoot
  (params (ActionValue :type Boolean) (ElapsedSeconds :type Float%20%28double-precision%29) (TriggeredSeconds :type Float%20%28double-precision%29) (InputAction :type Input%20Action%20Object%20Reference :default "/Game/Player/Input/IA_Shoot.IA_Shoot"))
  (bind (_atk _velocity _life _bulletclass _bulletcounts _scale _destroy_) (Utilities|GetBulletData))
  (bind _shootpoint (Variables|Default|GetShootPoint))
  (bind _returnvalue (Transformation|GetWorldRotation _shootpoint))
  ;[1 1 1] Shoot
  (switch Utilities|FlowControl|Switch|SwitchonEmu_Action (Variables|角色|GetEmu_Action)
    (:NewEnumerator0
      (switch Utilities|FlowControl|Switch|SwitchonEmu_ShootMode (Variables|Default|GetShootMode)
        (:NewEnumerator0
          (for _index (range 0 1) :!label _label
            (Game|SpawnActorfromClass "/Game/Player/BP_Player_Bullet_1.BP_Player_Bullet_1_C" (Math|Transform|MakeTransform (Utilities|Select :Index _index :Option%200 (Transformation|GetWorldLocation (Variables|Default|GetShootPoint1)) :Option%201 (Transformation|GetWorldLocation (Variables|Default|GetShootPoint2))) (Utilities|Select :Index _index :Option%200 (Transformation|GetWorldRotation (Variables|Default|GetShootPoint1)) :Option%201 (Transformation|GetWorldRotation (Variables|Default|GetShootPoint2))) "1.500000,1.500000,1.500000") "Undefined" "MultiplyWithRoot" 0 (Utilities|Select :Index (Variables|Default|GetShootMode) :NewEnumerator0 "(R=1.000000,G=1.000000,B=1.000000,A=1.000000)" :NewEnumerator1 "(R=1.000000,G=0.041492,B=0.000000,A=1.000000)") "1000.000000,0.000000,0.000000" (Variables|角色|GetATK) 0.0 "NewEnumerator3" true (Variables|Default|GetShootMode) 0))
          (for _index_2 (range 0 _bulletcounts)
            (bind _output_get (Variables|Bullet|SetBullet _bulletclass))
            (Game|SpawnActorfromClass _output_get (Math|Transform|MakeTransform (Transformation|GetWorldLocation _shootpoint) (Math|Rotator|MakeRotator (.roll _returnvalue) (+ (.pitch _returnvalue) (Utilities|Array|Get(acopy) (Variables|角色|GetShootAngle) _index_2)) (.yaw _returnvalue)) _scale) "Undefined" "MultiplyWithRoot" 0 (Utilities|Select :Index (Variables|Default|GetShootMode) :NewEnumerator0 "(R=1.000000,G=1.000000,B=1.000000,A=1.000000)" :NewEnumerator1 "(R=1.000000,G=0.041492,B=0.000000,A=1.000000)") _velocity _atk _life (Variables|Bullet|GetPlayerBullet) _destroy_ (Variables|Default|GetShootMode) 0)
            (Variables|角色|SetEmu_Action "NewEnumerator1")
            (Utilities|FlowControl|Delay (Variables|角色|GetShootRate))
            (Variables|角色|SetEmu_Action "NewEnumerator0")
            (switch Utilities|FlowControl|Switch|SwitchonEmu_ShootMode (Variables|Default|GetShootMode)
              (:NewEnumerator1
                (bind _returnvalue_2 (Utilities|Time|SetTimerbyEvent (delegate Custom|RefreshEp) 0.6 true))
                (Variables|Default|SetRefreshEp_Handle _returnvalue_2)))))
        (:NewEnumerator1
          (if (not (== (Variables|角色|GetEP) 0.0))
            (Utilities|UpdateEp)
            (goto _label)))))))

(event Input|EnhancedActionEvents|EnhancedInputActionIA_WL
  (params (ActionValue :type Boolean) (ElapsedSeconds :type Float%20%28double-precision%29) (TriggeredSeconds :type Float%20%28double-precision%29) (InputAction :type Input%20Action%20Object%20Reference :default "/Game/Player/Input/IA_WL.IA_WL"))
  ;[1 1 1] Shoot
  (:Started
    (bind _新建轨道_0 (Timeline|Wingman%20Rotate Play)
      (:Update
        (Transformation|SetRelativeRotation (Variables|Default|GetWingman_1) (Math|Rotator|Lerp(Rotator) "-90.000000,0.000000,0.000000" "90.000000,0.000000,0.000000" _新建轨道_0) false false)
        (Transformation|SetRelativeRotation (Variables|Default|GetWingman_2) (Math|Rotator|Lerp(Rotator) "-90.000000,0.000000,0.000000" "-270.000000,0.000000,0.000000" _新建轨道_0) false false))))
  (:Completed
    (Timeline|Wingman%20Rotate Stop)))

(event Input|EnhancedActionEvents|EnhancedInputActionIA_WR
  (params (ActionValue :type Boolean) (ElapsedSeconds :type Float%20%28double-precision%29) (TriggeredSeconds :type Float%20%28double-precision%29) (InputAction :type Input%20Action%20Object%20Reference :default "/Game/Player/Input/IA_WR.IA_WR"))
  ;[1 1 1] Shoot
  (:Started
    (bind _新建轨道_0 (Timeline|Wingman%20Rotate Reverse)
      (:Update
        (Transformation|SetRelativeRotation (Variables|Default|GetWingman_1) (Math|Rotator|Lerp(Rotator) "-90.000000,0.000000,0.000000" "90.000000,0.000000,0.000000" _新建轨道_0) false false)
        (Transformation|SetRelativeRotation (Variables|Default|GetWingman_2) (Math|Rotator|Lerp(Rotator) "-90.000000,0.000000,0.000000" "-270.000000,0.000000,0.000000" _新建轨道_0) false false))))
  (:Completed
    (Timeline|Wingman%20Rotate Stop)))

(event Input|EnhancedActionEvents|EnhancedInputActionIA_ShootMode
  (params (ActionValue :type Boolean) (ElapsedSeconds :type Float%20%28double-precision%29) (TriggeredSeconds :type Float%20%28double-precision%29) (InputAction :type Input%20Action%20Object%20Reference :default "/Game/Player/Input/IA_ShootMode.IA_ShootMode"))
  (:Started
    (Utilities|FlowControl|FlipFlop
      (:A
        (bind _output_get (Variables|Default|SetShootMode "NewEnumerator1"))
        (Default|SwitchShootMode (Variables|Default|GetUI_Player) _output_get))
      (:B
        (bind _output_get_2 (Variables|Default|SetShootMode "NewEnumerator0"))
        (Default|SwitchShootMode (Variables|Default|GetUI_Player) _output_get_2)))))

(fn ConstructionScript)

(fn UpdateUIHp
  (bind _ui_player (Variables|Default|GetUI_Player)
    (:then
      (Default|UpdateUIHp _ui_player (/ (Variables|Character|GetHP) (Variables|角色|GetHPMax))))
    (:else)))

(fn ActiveBullet
  (params (bullet :type Emu_PlayerBullet%20Enum :default "NewEnumerator0"))
  (if (not (.ReturnValue (Utilities|Map|Find (Variables|Bullet|GetPlayerBulletLevel) bullet)))
    (Utilities|Map|Add (Variables|Bullet|GetPlayerBulletLevel) bullet 1)
    (Utilities|Map|Add (Variables|Bullet|GetPlayerBulletExp) bullet 0)
    (bind _ui_player (Variables|Default|GetUI_Player)
      (:then
        (Default|ActiveUIBullet _ui_player bullet))
      (:else))))

(fn UpdateBulletExpandLevel
  (params (GetBullet :type Emu_PlayerBullet%20Enum%20%28by%20ref%29 :default "NewEnumerator0"))
  (bind _bulletexp (Variables|Bullet|GetBulletExp))
  (bind _playerbulletlevel (Variables|Bullet|GetPlayerBulletLevel))
  (bind _playerbulletlevel_2 (Variables|Bullet|GetPlayerBulletLevel))
  (bind _playerbulletexp (Variables|Bullet|GetPlayerBulletExp))
  (bind _value (Utilities|Map|Find _playerbulletexp GetBullet))
  (bind (_value_2 _returnvalue) (Utilities|Map|Find _playerbulletlevel_2 GetBullet))
  (bind _returnvalue_2 (+ _value _bulletexp))
  (if _returnvalue
    (if (not (== _value_2 (Variables|Bullet|GetBulletLevelMax)))
      (if (>= _returnvalue_2 (Variables|Bullet|GetBulletLevelup))
        (Utilities|Map|Add (Variables|Bullet|GetPlayerBulletExp) GetBullet 0)
        (bind _result (Math|Integer|IncrementInt (.Value (Utilities|Map|Find _playerbulletlevel GetBullet)))
          (:%20%20
            (Utilities|Map|Add _playerbulletlevel GetBullet _result)
            (Default|UpdateUIBulletLevel (Variables|Default|GetUI_Player) GetBullet (/ (Math|Conversions|ToFloat(Integer) _result) (Math|Conversions|ToFloat(Integer) (Variables|Bullet|GetBulletLevelMax))))
            (Default|UpdateUIBulletExp (Variables|Default|GetUI_Player) GetBullet 0.0)))
        (else
          (Utilities|Map|Add (Variables|Bullet|GetPlayerBulletExp) GetBullet _returnvalue_2)
          (Default|UpdateUIBulletExp (Variables|Default|GetUI_Player) GetBullet (/ (Math|Conversions|ToFloat(Integer) _returnvalue_2) (Math|Conversions|ToFloat(Integer) (Variables|Bullet|GetBulletLevelup)))))))))

(fn StartShield
  (params (Shield? :type Boolean))
  (Development|SetHiddeninGame (Variables|Default|GetShield_FB) (not Shield?) false)
  (Variables|Default|SetShield? Shield?))