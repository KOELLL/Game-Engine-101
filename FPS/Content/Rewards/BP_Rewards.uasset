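; BP_Rewards is a 2D flipbook pickup that drifts around the play area and grants a health, shield or one of three B-type rewards to the player.
; On spawn it launches in a random direction from a preset array via projectile movement, setting its flipbook and scale from the reward enum.
; Its box overlap flips X or Z velocity on tagged walls, and on "P"-tagged actors sends the reward message and destroys itself.
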(event OnComponentBeginOverlap(Box)
  (params (OverlappedComponent :type Primitive%20Component%20Object%20Reference) (OtherActor :type Actor%20Object%20Reference) (OtherComp :type Primitive%20Component%20Object%20Reference) (OtherBodyIndex :type Integer) (bFromSweep :type Boolean) (SweepResult :type Hit%20Result%20Structure%20%28by%20ref%29))
  (CallFunction|BoxOverlap OtherActor))

(event EventBeginPlay
  (Utilities|Init))

(fn ConstructionScript)

(fn BoxOverlap
  (params (Actor :type Actor%20Object%20Reference))
  (if (Actor|ActorHasTag Actor "Wall")
    (if (Actor|ActorHasTag Actor "LR")
      (Variables|Default|SetCurrentVelocity (Math|Vector|MakeVector (* (.x (Variables|Default|GetCurrentVelocity)) -1.0) (.y (Variables|Default|GetCurrentVelocity)) (.z (Variables|Default|GetCurrentVelocity))))
      (else
        (Variables|Default|SetCurrentVelocity (Math|Vector|MakeVector (.x (Variables|Default|GetCurrentVelocity)) (.y (Variables|Default|GetCurrentVelocity)) (* (.z (Variables|Default|GetCurrentVelocity)) -1.0)))))
    (Game|Components|ProjectileMovement|SetVelocityinLocalSpace (Variables|Default|GetProjectileMovement) (* (Variables|Default|GetCurrentVelocity) (Variables|Default|GetSpeed)))
    (elif (Actor|ActorHasTag Actor "P")
      (Class|IFPlayer|GetReward(Message) Actor (Variables|Default|GetEmu_Reward))
      (Actor|DestroyActor))))