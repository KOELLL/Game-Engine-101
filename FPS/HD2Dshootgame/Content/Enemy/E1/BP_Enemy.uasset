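; BP_Enemy is an enemy actor that configures its stats and idle animation from a data table at BeginPlay.
; Init caches the ABP_Enemy animation instance, then reads the DT_Enemy row named after the EmuEnemy enum value into health, SH, attack, life, speed and idle animation variables.
; It then hands the idle animation to the anim instance, so the enum value selects both stats and visuals.
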(event EventBeginPlay
  (Utilities|Init))

(fn ConstructionScript)