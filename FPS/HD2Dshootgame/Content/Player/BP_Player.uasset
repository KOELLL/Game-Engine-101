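; BP_Player is the player character, flown in the world X-Z plane while viewed through a separate BP_Camera actor.
; On BeginPlay it sets that camera as view target, disables capsule physics, adds the Enhanced Input mapping and caches the ABP_Player anim instance.
; IA_Move drives movement input and sets a fly-action enum from full up, full down or neutral vertical input, pushing it to the animation blueprint.
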(event EventBeginPlay
  (Utilities|Init))

(event Input|EnhancedActionEvents|EnhancedInputActionIA_Move
  (params (ActionValue :type Vector%202D%20Structure) (ElapsedSeconds :type Float%20%28double-precision%29) (TriggeredSeconds :type Float%20%28double-precision%29) (InputAction :type Input%20Action%20Object%20Reference :default "/Game/Player/Input/IA_Move.IA_Move"))
  (bind (_x _y) (Math|Vector2D|BreakVector2D ActionValue))
  ;[0.15 0.15 0.15 0.5] Move
  (:Triggered
    (Pawn|Input|AddMovementInput "1.000000,0.000000,0.000000" _x false)
    (Pawn|Input|AddMovementInput "0.000000,0.000000,1.000000" _y false)
    (if (== _y 1.0)
      (bind _output_get (Variables|Default|SetEnum_FlyAction "NewEnumerator1"))
      (Variables|/Game/Player/ABP_Player.ABP_Player_C|SetEnum_FlyAction (Variables|Default|GetAs%20ABP%20Player) _output_get)
      (elif (== _y -1.0)
        (bind _output_get_2 (Variables|Default|SetEnum_FlyAction "NewEnumerator2"))
        (Variables|/Game/Player/ABP_Player.ABP_Player_C|SetEnum_FlyAction (Variables|Default|GetAs%20ABP%20Player) _output_get_2)
        (else
          (bind _output_get_3 (Variables|Default|SetEnum_FlyAction "NewEnumerator0"))
          (Variables|/Game/Player/ABP_Player.ABP_Player_C|SetEnum_FlyAction (Variables|Default|GetAs%20ABP%20Player) _output_get_3)))))
  (:Completed
    (bind _output_get_4 (Variables|Default|SetEnum_FlyAction "NewEnumerator0"))
    (Variables|/Game/Player/ABP_Player.ABP_Player_C|SetEnum_FlyAction (Variables|Default|GetAs%20ABP%20Player) _output_get_4)))

(fn ConstructionScript)