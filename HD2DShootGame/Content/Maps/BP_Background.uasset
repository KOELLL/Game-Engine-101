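; Background actor that shows a configurable texture on a plane with a time-animated material.
; The construction script creates a dynamic instance of M_Background_Inst, applies it to the plane and passes in the texture, brightness, Op and X/Y/U/V variables.
; Tick accumulates delta time scaled by Speed and writes it to the material's Time parameter, so the material drives the animation at an adjustable rate.
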(event EventBeginPlay)

(event Collision|EventActorBeginOverlap
  (params (OtherActor :type Actor%20Object%20Reference)))

(event EventTick
  (params (DeltaSeconds :type Float%20%28single-precision%29))
  (bind _output_get (Variables|Default|Settime (+ (* DeltaSeconds (Variables|Default|Getspeed)) (Variables|Default|Gettime))))
  (Rendering|Material|SetScalarParameterValue (Variables|Default|GetM) "Time" _output_get :!class /Script/Engine.MaterialInstanceDynamic))

(fn ConstructionScript
  (bind _returnvalue (Rendering|Material|CreateDynamicMaterialInstance "/Game/Material/M_Background_Inst.M_Background_Inst" "None" "None" :!class /Script/Engine.KismetMaterialLibrary))
  (bind _output_get (Variables|Default|SetM _returnvalue))
  (Rendering|Material|SetMaterial (Variables|Default|GetPlane) 0 _output_get)
  (Rendering|Material|SetTextureParameterValue (Variables|Default|GetM) "Texture" (Variables|Default|Gettexture))
  (Rendering|Material|SetScalarParameterValue (Variables|Default|GetM) "Brightness" (Variables|Default|Getbrightness) :!class /Script/Engine.MaterialInstanceDynamic)
  (Rendering|Material|SetScalarParameterValue (Variables|Default|GetM) "Op" (Variables|Default|GetOp) :!class /Script/Engine.MaterialInstanceDynamic)
  (Rendering|Material|SetScalarParameterValue (Variables|Default|GetM) "x" (Variables|Default|Getx) :!class /Script/Engine.MaterialInstanceDynamic)
  (Rendering|Material|SetScalarParameterValue (Variables|Default|GetM) "y" (Variables|Default|Gety) :!class /Script/Engine.MaterialInstanceDynamic)
  (Rendering|Material|SetScalarParameterValue (Variables|Default|GetM) "u" (Variables|Default|Getu) :!class /Script/Engine.MaterialInstanceDynamic)
  (Rendering|Material|SetScalarParameterValue (Variables|Default|GetM) "v" (Variables|Default|Getv) :!class /Script/Engine.MaterialInstanceDynamic))